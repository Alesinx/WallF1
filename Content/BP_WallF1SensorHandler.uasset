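; BP_WallF1SensorHandler bridges a wall sensor handler to MQTT messaging through publish and subscribe events.
; BPPublish and BPSubscribe forward topic, payload and QoS arguments to an existing MqttClient, printing an error when it is invalid.
; Each subscription binds a message handler that relays incoming messages to OnMessageReceived, whose logic lies outside this graph.
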(event Custom|CustomEvent
  (params (Message :type MQTT%20Client%20Message%20Structure%20%28by%20ref%29))
  (Class|WallF1SensorHandler|OnMessageReceived Message))

(event EventBPPublish
  (params (InTopic :type String) (InPayload :type Array%20of%20Bytes) (InQoS :type EMQTTQualityOfService%20Enum :default "Once") (bInRetain :type Boolean))
  (bind _mqttclient (Variables|Default|GetMqttClient))
  (Utilities|IsValid _mqttclient
    (:Is%20Valid
      (Class|MQTTClientObject|Publish _mqttclient InTopic InPayload InQoS false))
    (:Is%20Not%20Valid
      (Development|PrintString 0 "MqttClient was null!" true true "(R=1.000000,G=0.000000,B=0.000000,A=1.000000)"))))

(event EventBPSubscribe
  (params (InTopic :type String) (InQoS :type EMQTTQualityOfService%20Enum :default "Once"))
  (bind _mqttclient (Variables|Default|GetMqttClient))
  (Utilities|IsValid _mqttclient
    (:Is%20Valid
      (bind _returnvalue (Class|MQTTClientObject|Subscribe _mqttclient InTopic InQoS))
      (Class|MQTTSubscriptionObject|SetonMessageHandler _returnvalue (delegate Custom|CustomEvent)))
    (:Is%20Not%20Valid
      (Development|PrintString 0 "MqttClient was null!" true true "(R=1.000000,G=0.000000,B=0.000000,A=1.000000)"))))